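; Score display actor for the indoor shooting range that shows a points value on a TextRender component.
; The Pontos function stores the incoming value in Pontos0, writes it to the text and always returns zero.
; Tick feeds the stored value back through that function, then sets the text to the returned value, so the display is overwritten with zero every frame.
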(event EventTick
  (params (DeltaSeconds :type Float%20%28single-precision%29))
  (bind _newparam (CallFunction|Pontos (Variables|Default|GetPontos_0)))
  (Rendering|Components|TextRender|SetText (Variables|Default|GetTextRender) (Utilities|Text|ToText(Float) _newparam "HalfToEven")))

(fn ConstructionScript)

(fn Pontos
  (params (Pontos :type Float%20%28double-precision%29%20%28by%20ref%29))
  (bind _output_get (Variables|Default|SetPontos_0 Pontos))
  (Rendering|Components|TextRender|SetText (Variables|Default|GetTextRender) (Utilities|Text|ToText(Float) _output_get "HalfToEven"))
  (return 0.0))